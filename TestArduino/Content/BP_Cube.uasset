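; BP_Cube is an actor whose rotation is driven by orientation data received over UDP.
; On BeginPlay it opens a receive socket on a hardcoded local address and port, binds a bytes-received event, and caches the first BP_Cube found in the level.
; Each packet is printed and parsed as JSON, and its roll, pitch and yaw set that cube's rotation.
; EndPlay closes the socket.
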(event `self.ReceiveBeginPlay`
  (bind _udp (`self.UDP`))
  (`UDPComponent.OpenReceiveSocket` _udp "192.168.1.2" 3002)
  (add `UDPComponent.OnReceivedBytes` _udp (delegate `UDPReceivedEvent`))
  (bind _returnvalue (`GameplayStatics.GetActorOfClass` "BP_Cube_C")))

(event `self.ReceiveEndPlay`
  (params (EndPlayReason :type "EEndPlayReason Enum" :default "Destroyed"))
  (`UDPComponent.CloseReceiveSocket` (`self.UDP`)))

(event `UDPReceivedEvent`
  (params (Bytes :type "Array of Byte (by ref)") (IPAddress :type String))
  (bind _returnvalue (`CUBlueprintLibrary.Conv_BytesToString` Bytes))
  (bind _returnvalue_2 (`SIOJLibrary.Conv_JsonValueToJsonObject` (`SIOJsonValue.ValueFromJsonString` _returnvalue)))
  (`KismetSystemLibrary.PrintString` _returnvalue)
  (`self.K2_SetActorRotation` (stale `self.ReceiveBeginPlay` _returnvalue) (`KismetMathLibrary.MakeRotator` (`SIOJsonObject.GetNumberField` _returnvalue_2 "roll") (`SIOJsonObject.GetNumberField` _returnvalue_2 "pitch") (`SIOJsonObject.GetNumberField` _returnvalue_2 "yaw")) false))

(fn `UserConstructionScript`)